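; JobBP is a job trigger that pays the player for a work shift.
; A box overlap while the main character's Hours are 8 to 11 shows a JobWB widget, adds random Money and jumps the clock to a random evening time.
; It calls SetIgnoreMoveInput with false, so movement is not blocked, then resets move input after a short delay.
; The overlapping actor is never checked.
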(event OnComponentBeginOverlap(Box)
  (params (OverlappedComponent :type Primitive%20Component%20Object%20Reference) (OtherActor :type Actor%20Object%20Reference) (OtherComp :type Primitive%20Component%20Object%20Reference) (OtherBodyIndex :type Integer) (bFromSweep :type Boolean) (SweepResult :type Hit%20Result%20Structure%20%28by%20ref%29))
  (bind _returnvalue (Game|GetPlayerController 0))
  (bind _as_main_character (Variables|Default|GetAs%20Main%20Character))
  (if (and (<= (Variables|/Game/Game/Character/MainCharacter.MainCharacter_C|GetHours _as_main_character) 11) (>= (Variables|/Game/Game/Character/MainCharacter.MainCharacter_C|GetHours _as_main_character) 8))
    (Input|SetIgnoreMoveInput _returnvalue false)
    (bind _returnvalue_2 (UserInterface|CreateWidget "/Game/GameUI/MainGame/Interface/JobWB.JobWB_C"))
    (UserInterface|Viewport|AddtoViewport _returnvalue_2 0)
    (Variables|/Game/Game/Character/MainCharacter.MainCharacter_C|SetMoney _as_main_character (+ (Variables|/Game/Game/Character/MainCharacter.MainCharacter_C|GetMoney _as_main_character) (Math|Random|RandomIntegerinRange 120 300)))
    (bind _asmain_character (Utilities|Casting|CastToMainCharacter (Game|GetPlayerCharacter 0)))
    (Variables|/Game/Game/Character/MainCharacter.MainCharacter_C|SetHours _asmain_character (Math|Random|RandomIntegerinRange 17 19))
    (Variables|/Game/Game/Character/MainCharacter.MainCharacter_C|SetMinutes _asmain_character (Math|Random|RandomIntegerinRange 10 43))
    (Utilities|FlowControl|Delay 5.0)
    (Input|ResetIgnoreMoveInput _returnvalue)))

(event EventBeginPlay
  (bind _asmain_character (Utilities|Casting|CastToMainCharacter (Game|GetPlayerCharacter 0)))
  (Variables|Default|SetAs%20Main%20Character _asmain_character))

(fn ConstructionScript)