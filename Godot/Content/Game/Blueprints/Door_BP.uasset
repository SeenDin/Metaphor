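; Interactable door Blueprint that swings open and closed by rotating its Scene component around yaw.
; The Interact event branches on a boolean, НАПерсонажа ("toward the character"), to pick one of two timelines, presumably for opposite swing directions.
; Each branch has its own FlipFlop that alternates playing and reversing its timeline, whose Open track sets the relative yaw.
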(event EventInteract
  (bind _scene (Variables|Default|GetScene))
  (if (Variables|Default|GetНА%20персонажа?)
    (Utilities|FlowControl|FlipFlop
      (:A
        (bind _open (Timeline|Open Play)
          (:Update
            (Transformation|SetRelativeRotation _scene (Math|Rotator|MakeRotator 0.0 0.0 _open) false false))))
      (:B
        (Timeline|Open Reverse)))
    (else
      (Utilities|FlowControl|FlipFlop
        (:A
          (bind _open_2 (Timeline|Timeline Play)
            (:Update
              (Transformation|SetRelativeRotation _scene (Math|Rotator|MakeRotator 0.0 0.0 _open_2) false false))))
        (:B
          (Timeline|Timeline Reverse))))))

(fn ConstructionScript)