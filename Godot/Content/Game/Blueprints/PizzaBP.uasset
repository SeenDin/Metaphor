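; PizzaBP is an interactable pizza pickup that the player eats to reduce hunger.
; On BeginPlay it casts the player pawn to MainCharacter and caches the reference.
; On Interact, if the character's Hunge value is above zero, it subtracts a fixed amount with no clamp and destroys itself.
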(event EventInteract
  (bind _as_main_character (Variables|Default|GetAs%20Main%20Character))
  (if (> (Variables|/Game/Game/Character/MainCharacter.MainCharacter_C|GetHunge _as_main_character) 0)
    (Variables|/Game/Game/Character/MainCharacter.MainCharacter_C|SetHunge _as_main_character (- (Variables|/Game/Game/Character/MainCharacter.MainCharacter_C|GetHunge _as_main_character) 20))
    (Actor|DestroyActor)))

(event EventBeginPlay
  (bind _asmain_character (Utilities|Casting|CastToMainCharacter (Game|Player|GetPlayerPawn 0)))
  (Variables|Default|SetAs%20Main%20Character _asmain_character))

(fn ConstructionScript)