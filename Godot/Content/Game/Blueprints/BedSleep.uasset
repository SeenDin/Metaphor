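; BedSleep is an interactable bed that lets the player sleep through the night once the in-game hour is past 17.
; Interacting shows the SleepInBedWB widget, increments the day on MainCharacter and sets a randomized morning time.
; It calls SetIgnoreMoveInput with false, which does not block movement, then resets move-input ignoring after a five-second delay.
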(event EventBeginPlay
  (bind _asmain_character (Utilities|Casting|CastToMainCharacter (Game|GetPlayerCharacter 0)))
  (Variables|Default|SetAs%20Main%20Character _asmain_character))

(event EventInteract
  (bind _returnvalue (Game|GetPlayerController 0))
  (bind _as_main_character (Variables|Default|GetAs%20Main%20Character))
  (if (not (<= (Variables|/Game/Game/Character/MainCharacter.MainCharacter_C|GetHours (Variables|Default|GetAs%20Main%20Character)) 17))
    (Input|SetIgnoreMoveInput _returnvalue false)
    (bind _returnvalue_2 (UserInterface|CreateWidget "/Game/GameUI/MainGame/Interface/SleepInBedWB.SleepInBedWB_C"))
    (UserInterface|Viewport|AddtoViewport _returnvalue_2 0)
    (bind _result (Math|Integer|IncrementInt (Variables|/Game/Game/Character/MainCharacter.MainCharacter_C|GetDay _as_main_character))
      (:%20%20
        (Variables|/Game/Game/Character/MainCharacter.MainCharacter_C|SetDay _as_main_character _result)
        (Variables|/Game/Game/Character/MainCharacter.MainCharacter_C|SetHours _as_main_character (Math|Random|RandomIntegerinRange 7 8))
        (Variables|/Game/Game/Character/MainCharacter.MainCharacter_C|SetMinutes _as_main_character (Math|Random|RandomIntegerinRange 0 53))
        (Utilities|FlowControl|Delay 5.0)
        (Input|ResetIgnoreMoveInput _returnvalue)))))

(fn ConstructionScript)